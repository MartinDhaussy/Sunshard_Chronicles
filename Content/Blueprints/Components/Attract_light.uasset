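; A light component that lures BP_Mutants toward itself while activated.
; Each tick it sphere-overlaps pawns within its attenuation radius and line-traces on Visibility to each mutant.
; Mutants with an unblocked trace get an AdvancedMoveTo toward the light's navmesh-projected position, or its raw location if projection fails.
; A debug sphere draw for the radius exists but is disconnected.
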(event `self.ReceiveTick`
  (params (DeltaSeconds :type "Float (single-precision)"))
  (bind _returnvalue (`self.K2_GetComponentLocation`))
  (bind (_projectedlocation _returnvalue_2) (`NavigationSystemV1.K2_ProjectPointToNavigation` _returnvalue null null (350.0 350.0 350.0)))
  (if (`self.Activated`)
    (`|ExecutionSequence`
      (:`then_0`
        (bind _outactors (`KismetSystemLibrary.SphereOverlapActors` (`self.K2_GetComponentLocation`) (`self.AttenuationRadius`) (`|MakeArray` "ObjectTypeQuery3" :!type "EObjectTypeQuery Enum") "/Script/Engine.Pawn"))
        (for _array_element _outactors
          (bind _asbp_mutants (cast `/Game/ThirdPerson/Blueprints/BP_Mutants` _array_element))
          (bind (_outhit _returnvalue_3) (`KismetSystemLibrary.LineTraceSingle` (`self.K2_GetComponentLocation`) (`Actor.K2_GetActorLocation` _asbp_mutants) "TraceTypeQuery1"))
          (if (not _returnvalue_3)
            (`/Game/ThirdPerson/Blueprints/BP_Mutants.AdvancedMoveTo` _asbp_mutants (`self.Acceptance Radius`) false null (select `bool` _returnvalue_2 :`false` _returnvalue :`true` _projectedlocation)))))
      (:`then_1`))))