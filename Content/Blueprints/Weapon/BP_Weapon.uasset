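; Pickup weapon that fires big or little projectiles by mode, building heat and a light-based attraction radius.
; Each shot spawns linked muzzle and camera projectiles, both aimed along camera rotation, with DoOnce-plus-Delay limiting fire rate.
; Tick decays heat and radius, driving an emissive material parameter and light attenuation; overheating blocks firing and triggers smoke and sound.
; Pickup overlap toggles a text prompt, which Interact hides after a delay.
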(event `Shoot`
  (params (Mode :type Integer) (attractlight :type "/Game/Blueprints/Components/Attract_light Object Reference") (`Fumée` :type "NiagaraComponent Object Reference"))
  (bind _returnvalue (`PlayerCameraManager.GetCameraRotation` (`GameplayStatics.GetPlayerCameraManager` 0)))
  (bind _returnvalue_2 (`PlayerCameraManager.GetCameraRotation` (`GameplayStatics.GetPlayerCameraManager` 0)))
  (bind _returnvalue_3 (`PlayerCameraManager.GetCameraRotation` (`GameplayStatics.GetPlayerCameraManager` 0)))
  (bind _returnvalue_4 (`PlayerCameraManager.GetCameraRotation` (`GameplayStatics.GetPlayerCameraManager` 0)))
  (set `self.Attractlight` attractlight)
  (if (not (`self.IsOverheating`))
    (switch `int` Mode
      (:`0`
        ;[1 1 1] Big Projectile
        (`/Engine/EditorBlueprintResources/StandardMacros.DoOnce` false :!label _label
          (:`Completed`
            (`|ExecutionSequence`
              (:`then_0`
                (`self.AddHeat` 0.5)
                (`self.Attract_Radius` 500.0)
                (bind _returnvalue_5 (`|SpawnActorFromClass` "/Game/Blueprints/Weapon/BP_BigProj.BP_BigProj_C" (`KismetMathLibrary.MakeTransform` (+ (`SceneComponent.GetSocketLocation` (`self.Muzzle`) "None") (`KismetMathLibrary.GreaterGreater_VectorRotator` (`self.Projectile Offset`) _returnvalue_3)) _returnvalue_3) "AlwaysSpawn" "MultiplyWithRoot" null null))
                (`KismetSystemLibrary.Delay` 1.0)
                (goto _label :!via `Reset`))
              (:`then_1`
                (bind _returnvalue_6 (`|SpawnActorFromClass` "/Game/Blueprints/Weapon/BP_BigProjcam.BP_BigProjcam_C" (`KismetMathLibrary.MakeTransform` (+ (`SceneComponent.GetSocketLocation` (`self.Cam`) "None") (`KismetMathLibrary.GreaterGreater_VectorRotator` (`self.Projectile Offset`) _returnvalue)) _returnvalue) "AlwaysSpawn" "MultiplyWithRoot" null null))
                (`GameplayStatics.PlaySoundAtLocation` "/Game/Martin/Son/Weapon/BigShot_Cue.BigShot_Cue" (`self.K2_GetActorLocation`) (struct) 1.0 1.0 0.0 null null null null)
                (`KismetSystemLibrary.Delay` 1.0)
                (goto _label :!via `Reset`))
              (:`then_2`
                (set `/Game/Blueprints/Weapon/BP_BigProj.otherProjectile` _returnvalue_6 _returnvalue_5))))))
      (:`1`
        ;[1 1 1] Little Projectile
        (`/Engine/EditorBlueprintResources/StandardMacros.DoOnce` false :!label _label_2
          (:`Completed`
            (`|ExecutionSequence`
              (:`then_0`
                (`self.AddHeat` 0.2)
                (`self.Attract_Radius` 200.0)
                (bind _returnvalue_7 (`|SpawnActorFromClass` "/Game/Blueprints/Weapon/BP_LittleProj.BP_LittleProj_C" (`KismetMathLibrary.MakeTransform` (+ (`SceneComponent.GetSocketLocation` (`self.Muzzle`) "None") (`KismetMathLibrary.GreaterGreater_VectorRotator` (`self.Projectile Offset`) _returnvalue_2)) _returnvalue_2) "AlwaysSpawn" "MultiplyWithRoot" null null))
                (`KismetSystemLibrary.Delay` 0.2)
                (goto _label_2 :!via `Reset`))
              (:`then_1`
                (bind _returnvalue_8 (`|SpawnActorFromClass` "/Game/Blueprints/Weapon/BP_LittleProjcam.BP_LittleProjcam_C" (`KismetMathLibrary.MakeTransform` (+ (`SceneComponent.GetSocketLocation` (`self.Cam`) "None") (`KismetMathLibrary.GreaterGreater_VectorRotator` (`self.Projectile Offset`) _returnvalue_4)) _returnvalue_4) "AlwaysSpawn" "MultiplyWithRoot" null null))
                (`GameplayStatics.PlaySoundAtLocation` "/Game/Martin/Son/Weapon/LittleShot_Cue.LittleShot_Cue" (`self.K2_GetActorLocation`) (struct) 1.0 1.0 0.0 null null null null)
                (`KismetSystemLibrary.Delay` 0.2)
                (goto _label_2 :!via `Reset`))
              (:`then_2`
                (set `/Game/Blueprints/Weapon/BP_LittleProj.otherProjectile` _returnvalue_8 _returnvalue_7)))))))))

(event `self.ReceiveTick`
  (params (DeltaSeconds :type "Float (single-precision)"))
  (bind _attractlight (`self.Attractlight`))
  (bind _returnvalue (`KismetMathLibrary.FClamp` (- (`self.OverHeating`) (* DeltaSeconds (`KismetMathLibrary.SelectFloat` (`self.HeatDecraseOverTimeIfOverheating`) (`self.HeatDecreaseOverTime`) (`self.IsOverheating`))))))
  ;[1 1 1] Overheat
  (`|ExecutionSequence`
    (:`then_0`
      (bind _output_get (set `self.OverHeating` _returnvalue))
      (`KismetMaterialLibrary.SetScalarParameterValue` "/Game/Materials/MP_emissiveHeat.MP_emissiveHeat" "Emissive_Heat" _returnvalue)
      (if (== _output_get 0.0)
        (set `self.IsOverheating` false)))
    (:`then_1`
      (bind _output_get_2 (set `self.Change Radius` (`KismetMathLibrary.FClamp` (- (`self.Change Radius`) (* DeltaSeconds (`KismetMathLibrary.SelectFloat` (`self.RadiusDecreaseifOverHeat`) (`self.RadiusDecreaseOvertime`) (`self.Detectable`)))) 0.0 1000.0)))
      (`/Engine/EditorBlueprintResources/StandardMacros.IsValid` _attractlight
        (:`Is Valid`
          (`LocalLightComponent.SetAttenuationRadius` _attractlight _output_get_2)
          (if (== _output_get_2 0.0)
            (set `self.Detectable` false)))))
    (:`then_2`
      (if (`self.IsOverheating`)
        (`/Engine/EditorBlueprintResources/StandardMacros.DoOnce` false :!label _label_3
          (:`Completed`
            (`ActorComponent.Activate` (stale `Shoot` `Fumée`) true)
            (`GameplayStatics.PlaySoundAtLocation` "/Game/Martin/Son/Character/surchauffe_Cue.surchauffe_Cue" (`self.K2_GetActorLocation`) (struct) 1.0 1.0 0.0 null null null null)))
        (else
          (goto _label_3 :!via `Reset`))))))

(event `/Game/Blueprints/Components/Interact_interface.interact`
  ;[1 1 1] Interact
  (`/Engine/EditorBlueprintResources/StandardMacros.DoOnce` false
    (:`Completed`
      (`KismetSystemLibrary.Delay` 2.0)
      (`SceneComponent.SetVisibility` (`self.TextRender`) false false))))

(event `self.Pickup-Radius.OnComponentBeginOverlap`
  (params (OverlappedComponent :type "PrimitiveComponent Object Reference") (OtherActor :type "Actor Object Reference") (OtherComp :type "PrimitiveComponent Object Reference") (OtherBodyIndex :type Integer) (bFromSweep :type Boolean) (SweepResult :type "HitResult Structure (by ref)"))
  ;[1 1 1] Interact
  (cast `/Game/ThirdPerson/Blueprints/BP_ThirdPersonCharacter` OtherActor)
  (`SceneComponent.SetHiddenInGame` (`self.TextRender`) false false))

(event `self.Pickup-Radius.OnComponentEndOverlap`
  (params (OverlappedComponent :type "PrimitiveComponent Object Reference") (OtherActor :type "Actor Object Reference") (OtherComp :type "PrimitiveComponent Object Reference") (OtherBodyIndex :type Integer))
  ;[1 1 1] Interact
  (cast `/Game/ThirdPerson/Blueprints/BP_ThirdPersonCharacter` OtherActor)
  (`SceneComponent.SetHiddenInGame` (`self.TextRender`) true false))

(fn `AddHeat`
  (params (`value to add` :type "Float (double-precision)" :default 0.2))
  (bind _output_get (set `self.OverHeating` (+ (`self.OverHeating`) `value to add`)))
  (if (>= _output_get 1.0)
    (set `self.IsOverheating` true)))

(fn `Attract_Radius`
  (params (`Change Radius` :type "Float (double-precision)"))
  (bind _output_get (set `self.Change Radius` (+ `Change Radius` (`self.Change Radius`))))
  (if (>= _output_get 1000.0)
    (set `self.Detectable` true)))

(fn `UserConstructionScript`)