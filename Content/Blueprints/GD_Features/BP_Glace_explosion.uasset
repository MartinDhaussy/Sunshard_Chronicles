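; Destructible ice block that breaks when hit by an actor tagged Plasma.
; A Cube component listens for the hit, then destroys itself and activates the GlaceExplo component.
; Separately, Tick enables collision damage on the ice block Geometry Collection whenever BulletDestroy is true; this graph never sets that flag.
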(event `self.ReceiveTick`
  (params (DeltaSeconds :type "Float (single-precision)"))
  (if (`self.BulletDestroy`)
    (`GeometryCollectionComponent.SetEnableDamageFromCollision` (`self.IceBlock_GeometryCollection`) true)))

(event `self.Cube.OnComponentHit`
  (params (HitComponent :type "PrimitiveComponent Object Reference") (OtherActor :type "Actor Object Reference") (OtherComp :type "PrimitiveComponent Object Reference") (NormalImpulse :type "Vector Structure") (Hit :type "HitResult Structure (by ref)"))
  (`/Engine/EditorBlueprintResources/StandardMacros.IsValid` OtherActor
    (:`Is Valid`
      (if (`self.ActorHasTag` OtherActor "Plasma")
        (`ActorComponent.K2_DestroyComponent` (`self.Cube`))
        (`ActorComponent.Activate` (`self.Glace_explo`) false)))))

(fn `UserConstructionScript`)