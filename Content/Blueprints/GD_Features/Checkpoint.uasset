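; Checkpoint actor that saves itself on the player character and restores the player to it on respawn.
; A box overlap by the third-person character sets this checkpoint once via DoOnce.
; RespawnPlayer moves the player to the capsule's transform, optionally spawns and equips a weapon when GiveGun is set, then respawns every mutant and resets all patrol-change triggers in the level.
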(event `RespawnPlayer`
  (params (Player :type "/Game/ThirdPerson/Blueprints/BP_ThirdPersonCharacter Object Reference"))
  (bind _capsule (`self.Capsule`))
  ;[1 1 1] Respawn Player
  (`self.K2_SetActorLocationAndRotation` Player (`SceneComponent.K2_GetComponentLocation` _capsule) (`SceneComponent.K2_GetComponentRotation` _capsule) false false)
  (`|ExecutionSequence`
    (:`then_0`
      (if (`self.GiveGun`)
        (bind _returnvalue (`|SpawnActorFromClass` "/Game/Blueprints/Weapon/BP_Weapon.BP_Weapon_C" (`self.GetTransform`) "AlwaysSpawn" "MultiplyWithRoot" null null))
        (`/Game/ThirdPerson/Blueprints/BP_ThirdPersonCharacter.EquipWeapon` Player _returnvalue)))
    (:`then_1`
      (bind _outactors (`GameplayStatics.GetAllActorsOfClass` "/Game/ThirdPerson/Blueprints/BP_Mutants.BP_Mutants_C"))
      (for _array_element _outactors
        (`/Game/ThirdPerson/Blueprints/BP_Mutants.respawnMutant` _array_element)))
    (:`then_2`
      (bind _outactors_2 (`GameplayStatics.GetAllActorsOfClass` "/Game/Blueprints/GD_Features/Trigger_ChangePatrol.Trigger_ChangePatrol_C"))
      (for _array_element_2 _outactors_2
        (`/Game/Blueprints/GD_Features/Trigger_ChangePatrol.ResetTrigger` _array_element_2)))))

(event `self.Box.OnComponentBeginOverlap`
  (params (OverlappedComponent :type "PrimitiveComponent Object Reference") (OtherActor :type "Actor Object Reference") (OtherComp :type "PrimitiveComponent Object Reference") (OtherBodyIndex :type Integer) (bFromSweep :type Boolean) (SweepResult :type "HitResult Structure (by ref)"))
  ;[1 1 1] Trigger Checkpoint
  (bind _asbp_third_person_character (cast `/Game/ThirdPerson/Blueprints/BP_ThirdPersonCharacter` OtherActor))
  (`/Engine/EditorBlueprintResources/StandardMacros.DoOnce` false
    (:`Completed`
      (`/Game/ThirdPerson/Blueprints/BP_ThirdPersonCharacter.SetCheckpoint` _asbp_third_person_character self))))

(fn `UserConstructionScript`)