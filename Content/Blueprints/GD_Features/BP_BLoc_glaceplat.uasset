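; Flat ice block that melts away when a Plasma-tagged actor hits its Cube, destroying that actor on impact.
; The Fondre timeline drives two dissolve scalar parameters on the Cube's materials while eight Niagara effects activate.
; Delays started from the timeline update later destroy the effects and the Cube, then set the shared MP_AmountDissolve parameter collection to fully dissolved values.
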(event `self.ReceiveBeginPlay`)

(event `self.Cube.OnComponentHit`
  (params (HitComponent :type "PrimitiveComponent Object Reference") (OtherActor :type "Actor Object Reference") (OtherComp :type "PrimitiveComponent Object Reference") (NormalImpulse :type "Vector Structure") (Hit :type "HitResult Structure (by ref)"))
  (bind _cube (`self.Cube`))
  (bind _niagara (`self.Niagara`))
  (`/Engine/EditorBlueprintResources/StandardMacros.IsValid` OtherActor
    (:`Is Valid`
      (if (`self.ActorHasTag` OtherActor "Plasma")
        (`self.K2_DestroyActor` OtherActor)
        (bind (_direction _dissolve _dissolvetb) (`Timeline|Fondre`)
          (:`Update`
            (`/Engine/EditorBlueprintResources/StandardMacros.IsValid` _cube
              (:`Is Valid`
                (`MeshComponent.SetScalarParameterValueOnMaterials` _cube "Amount" (`KismetMathLibrary.Lerp` 0.0 1.1 _dissolve))
                (`MeshComponent.SetScalarParameterValueOnMaterials` _cube "AmountTB" (`KismetMathLibrary.Lerp` 0.0 1.25 _dissolvetb))
                (`|ExecutionSequence`
                  (:`then_0`
                    (`KismetSystemLibrary.Delay` 4.0)
                    (`ActorComponent.K2_DestroyComponent` (`self.Cube`))
                    (`KismetMaterialLibrary.SetScalarParameterValue` "/Game/Materials/MP_AmountDissolve.MP_AmountDissolve" "AmountDissolve" 1.1)
                    (`KismetMaterialLibrary.SetScalarParameterValue` "/Game/Materials/MP_AmountDissolve.MP_AmountDissolve" "AmountDissolveTB" 1.25))
                  (:`then_1`
                    (`/Engine/EditorBlueprintResources/StandardMacros.IsValid` _niagara
                      (:`Is Valid`
                        (`ActorComponent.Activate` _niagara false)
                        (`ActorComponent.Activate` (`self.Niagara1`) false)
                        (`ActorComponent.Activate` (`self.Niagara2`) false)
                        (`ActorComponent.Activate` (`self.Niagara3`) false)
                        (`ActorComponent.Activate` (`self.Niagara4`) false)
                        (`ActorComponent.Activate` (`self.Niagara5`) false)
                        (`ActorComponent.Activate` (`self.Niagara6`) false)
                        (`ActorComponent.Activate` (`self.Niagara7`) false)
                        (`KismetSystemLibrary.Delay` 3.0)
                        (`ActorComponent.K2_DestroyComponent` _niagara)
                        (`ActorComponent.K2_DestroyComponent` (`self.Niagara1`))
                        (`ActorComponent.K2_DestroyComponent` (`self.Niagara2`))
                        (`ActorComponent.K2_DestroyComponent` (`self.Niagara3`))
                        (`ActorComponent.K2_DestroyComponent` (`self.Niagara4`))
                        (`ActorComponent.K2_DestroyComponent` (`self.Niagara5`))
                        (`ActorComponent.K2_DestroyComponent` (`self.Niagara6`))
                        (`ActorComponent.K2_DestroyComponent` (`self.Niagara7`))))))))))))))

(fn `UserConstructionScript`)