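; Trigger actor that switches a BP_Mutants enemy to a new patrol when a BP_ThirdPersonCharacter overlaps it.
; The overlap passes a DoOnce gate, then calls ChangePatrol on EnemyActor with NewPatrol.
; ResetTrigger re-arms the gate.
; The construction script rebuilds a world-space spline linking the trigger to both the patrol and the enemy when both references are valid.
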(event `self.ReceiveActorBeginOverlap`
  (params (OtherActor :type "Actor Object Reference"))
  (cast `/Game/ThirdPerson/Blueprints/BP_ThirdPersonCharacter` OtherActor)
  (`/Engine/EditorBlueprintResources/StandardMacros.DoOnce` false :!label _label
    (:`Completed`
      (bind _asbp_mutants (cast `/Game/ThirdPerson/Blueprints/BP_Mutants` (`self.EnemyActor`)))
      (`/Game/ThirdPerson/Blueprints/BP_Mutants.ChangePatrol` _asbp_mutants (`self.NewPatrol`)))))

(event `ResetTrigger`
  (goto _label :!via `Reset`))

(fn `UserConstructionScript`
  (bind _returnvalue (`self.K2_GetActorLocation`))
  (bind _enemyactor (`self.EnemyActor`))
  (bind _newpatrol (`self.NewPatrol`))
  (bind _spline (`self.Spline`))
  (`SplineComponent.ClearSplinePoints` _spline true)
  (`/Engine/EditorBlueprintResources/StandardMacros.IsValid` _enemyactor
    (:`Is Valid`
      (`/Engine/EditorBlueprintResources/StandardMacros.IsValid` _newpatrol
        (:`Is Valid`
          (`SplineComponent.SetSplinePoints` _spline (`|MakeArray` _returnvalue (`self.K2_GetActorLocation` _newpatrol) _returnvalue (`self.K2_GetActorLocation` _enemyactor)) "World" true))))))