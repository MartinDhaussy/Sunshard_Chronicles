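; Burnable rope rig (corde) whose sphere drops as a temporary light source when a Fire_Bead hits the rope.
; The hit destroys bead, rope and collider, gives the sphere a flame material and physics, and activates PatrolOverride, which is also activated at BeginPlay.
; On overlap the sphere freezes, loses collision, triggers Niagara and enables its LightSourceComponent, which switches off after a delay as the combustible material is applied.
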(event `self.ReceiveBeginPlay`
  (`ActorComponent.SetActive` (`self.Patrol_Override`) true false))

(event `self.collider_corde.OnComponentHit`
  (params (HitComponent :type "PrimitiveComponent Object Reference") (OtherActor :type "Actor Object Reference") (OtherComp :type "PrimitiveComponent Object Reference") (NormalImpulse :type "Vector Structure") (Hit :type "HitResult Structure (by ref)"))
  (`/Engine/EditorBlueprintResources/StandardMacros.IsValid` OtherActor
    (:`Is Valid`
      (if (`self.ActorHasTag` OtherActor "Fire_Bead")
        (`ActorComponent.K2_DestroyComponent` (`self.collider_corde`))
        (`self.K2_DestroyActor` OtherActor)
        (`ActorComponent.K2_DestroyComponent` (`self.corde`))
        (`PrimitiveComponent.SetMaterial` (`self.Sphere`) 0 "/Game/Materials/MI_Flame.MI_Flame")
        (`|ExecutionSequence`
          (:`then_0`
            (`PrimitiveComponent.SetSimulatePhysics` (`self.Sphere`) true))
          (:`then_1`
            (`ActorComponent.SetActive` (`self.Patrol_Override`) true false)))))))

(event `self.Sphere.OnComponentBeginOverlap`
  (params (OverlappedComponent :type "PrimitiveComponent Object Reference") (OtherActor :type "Actor Object Reference") (OtherComp :type "PrimitiveComponent Object Reference") (OtherBodyIndex :type Integer) (bFromSweep :type Boolean) (SweepResult :type "HitResult Structure (by ref)"))
  (`|ExecutionSequence`
    (:`then_0`
      (`PrimitiveComponent.SetSimulatePhysics` (`self.Sphere`) false)
      (set `/Game/Blueprints/Components/Attract_light.Activated` true (`self.LightSourceComponent`))
      (`KismetSystemLibrary.Delay` 5.0)
      (set `/Game/Blueprints/Components/Attract_light.Activated` false (`self.LightSourceComponent`))
      (`PrimitiveComponent.SetMaterial` (`self.Sphere`) 0 "/Game/Materials/MI_Combustilbe.MI_Combustilbe"))
    (:`then_1`
      (`ActorComponent.Activate` (`self.Niagara`) false)
      (`PrimitiveComponent.SetCollisionEnabled` (`self.Sphere`) "NoCollision"))))

(fn `UserConstructionScript`)