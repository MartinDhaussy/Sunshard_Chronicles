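; BP_Brasier is a brazier that lights up when an actor tagged Fire_Bead overlaps its Flamed component.
; The first hit, gated by a DoOnce, plays the ignition sound at the base, shows the flame and its two light components, and sets LightSourceComponent to Activated.
; Every tagged bead is destroyed on overlap, including those arriving after the brazier is lit.
; The graph has no path to extinguish or reset it.
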(event `self.Flamed.OnComponentBeginOverlap`
  (params (OverlappedComponent :type "PrimitiveComponent Object Reference") (OtherActor :type "Actor Object Reference") (OtherComp :type "PrimitiveComponent Object Reference") (OtherBodyIndex :type Integer) (bFromSweep :type Boolean) (SweepResult :type "HitResult Structure (by ref)"))
  (`/Engine/EditorBlueprintResources/StandardMacros.IsValid` OtherActor
    (:`Is Valid`
      (if (`self.ActorHasTag` OtherActor "Fire_Bead")
        (`|ExecutionSequence`
          (:`then_0`
            (`/Engine/EditorBlueprintResources/StandardMacros.DoOnce` false
              (:`Completed`
                (`GameplayStatics.PlaySoundAtLocation` "/Game/Martin/Son/Brasier/BrasierUp_Cue.BrasierUp_Cue" (`SceneComponent.K2_GetComponentLocation` (`self.base`)) (struct) 1.0 1.0 0.0 null null null null)
                (`SceneComponent.SetVisibility` (`self.Flamme`) true false)
                (`SceneComponent.SetVisibility` (`self.Flame_light`) true false)
                (`SceneComponent.SetVisibility` (`self.Flame_volu`) true false)
                (set `/Game/Blueprints/Components/Attract_light.Activated` true (`self.LightSourceComponent`)))))
          (:`then_1`
            (`self.K2_DestroyActor` OtherActor)))))))

(fn `UserConstructionScript`)