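; Drawbridge (pont-levis) actor for Level 1 that is triggered when a Plasma-tagged actor hits its Box.
; The hit activates the ExploGlace effect, destroys the hitting actor and plays the Rotation timeline.
; The timeline drives the Cylinder's relative location and its roll and pitch, with yaw held at zero.
; Nothing in the graph reverses the motion.
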(event `self.Box.OnComponentHit`
  (params (HitComponent :type "PrimitiveComponent Object Reference") (OtherActor :type "Actor Object Reference") (OtherComp :type "PrimitiveComponent Object Reference") (NormalImpulse :type "Vector Structure") (Hit :type "HitResult Structure (by ref)"))
  (`/Engine/EditorBlueprintResources/StandardMacros.IsValid` OtherActor
    (:`Is Valid`
      (if (`self.ActorHasTag` OtherActor "Plasma")
        (`ActorComponent.Activate` (`self.Explo_glace`) false)
        (`self.K2_DestroyActor` OtherActor)
        (bind (_direction _position _rotationx _rotationy) (`Timeline|Rotation`)
          (:`Update`
            (`SceneComponent.K2_SetRelativeLocationAndRotation` (`self.Cylinder`) _position (`KismetMathLibrary.MakeRotator` (.x (`KismetMathLibrary.MakeVector` _rotationx _rotationy)) (.y (`KismetMathLibrary.MakeVector` _rotationx _rotationy))) false false)))))))

(fn `UserConstructionScript`)