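; BP_GlaceExplo_v2_2 is a Level 1 ice block that breaks apart when hit by plasma.
; A hit on the P1 block by an actor tagged Plasma destroys that component and activates the ExploGlace effect.
; Separately, Tick enables collision damage on the P2 geometry collection every frame while BulletDestroy is true.
; The file never sets BulletDestroy itself.
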(event `self.ReceiveTick`
  (params (DeltaSeconds :type "Float (single-precision)"))
  (if (`self.BulletDestroy`)
    (`GeometryCollectionComponent.SetEnableDamageFromCollision` (`self.BlocGlaceV2_P2_GeometryCollection`) true)))

(event `self.BlocGlaceV2_P1.OnComponentHit`
  (params (HitComponent :type "PrimitiveComponent Object Reference") (OtherActor :type "Actor Object Reference") (OtherComp :type "PrimitiveComponent Object Reference") (NormalImpulse :type "Vector Structure") (Hit :type "HitResult Structure (by ref)"))
  (`/Engine/EditorBlueprintResources/StandardMacros.IsValid` OtherActor
    (:`Is Valid`
      (if (`self.ActorHasTag` OtherActor "Plasma")
        (`ActorComponent.K2_DestroyComponent` (`self.BlocGlaceV2_P1`))
        (`ActorComponent.Activate` (`self.Explo_Glace`) false)))))

(fn `UserConstructionScript`)