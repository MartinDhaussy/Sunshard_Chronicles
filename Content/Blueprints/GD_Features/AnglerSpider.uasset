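; AnglerSpider is a patrolling hazard pawn that deals damage to any actor that overlaps it.
; On BeginPlay, a valid CurrentPatrolPoint becomes its target and switches on its AttractLight.
; Tick steers it toward the target through FloatingPawnMovement.
; Within ReachRadius of a PatrolPoint, it waits that point's WaitDuration via a Delay, then follows the linked NextPoint.
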(event `self.ReceiveActorBeginOverlap`
  (params (OtherActor :type "Actor Object Reference"))
  (`GameplayStatics.ApplyDamage` OtherActor 1.0 null self))

(event `self.ReceiveBeginPlay`
  (bind _current_patrol_point (`self.Current Patrol Point`))
  (`/Engine/EditorBlueprintResources/StandardMacros.IsValid` _current_patrol_point
    (:`Is Valid`
      (set `self.TargetActor` _current_patrol_point)
      (set `/Game/Blueprints/Components/Attract_light.Activated` true (`self.Attract_light`)))))

(event `self.ReceiveTick`
  (params (DeltaSeconds :type "Float (single-precision)"))
  (bind _returnvalue (`self.K2_GetActorLocation`))
  (bind _targetactor (`self.TargetActor`))
  (bind _returnvalue_2 (`self.K2_GetActorLocation` _targetactor))
  (`/Engine/EditorBlueprintResources/StandardMacros.IsValid` _targetactor
    (:`Is Valid`
      (`PawnMovementComponent.AddInputVector` (`self.FloatingPawnMovement`) (`KismetMathLibrary.Vector_ClampSizeMax` (- _returnvalue_2 _returnvalue) 1.0) false)
      (if (<= (`KismetMathLibrary.Vector_Distance` _returnvalue_2 _returnvalue) (`self.ReachRadius`))
        (bind _aspatrol_point (cast `/Game/ThirdPerson/Blueprints/PatrolPoint` (`self.TargetActor`)))
        (`KismetSystemLibrary.Delay` (`/Game/ThirdPerson/Blueprints/PatrolPoint.WaitDuration` _aspatrol_point))
        (set `self.TargetActor` (`/Game/ThirdPerson/Blueprints/PatrolPoint.NextPoint` _aspatrol_point))))))

(fn `UserConstructionScript`)