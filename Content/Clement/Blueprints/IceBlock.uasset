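; IceBlock is a destructible ice block that shatters when hit by an actor tagged Plasma.
; On the first such hit it destroys its static mesh, then reveals a geometry collection and enables its physics.
; A radial falloff field, placed at the hit point converted to actor-local space, applies external cluster strain to fracture the collection.
; A debug sphere is drawn using that same local position and the falloff radius.
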(event `self.StaticMesh.OnComponentHit`
  (params (HitComponent :type "PrimitiveComponent Object Reference") (OtherActor :type "Actor Object Reference") (OtherComp :type "PrimitiveComponent Object Reference") (NormalImpulse :type "Vector Structure") (Hit :type "HitResult Structure (by ref)"))
  (bind _geometrycollection (`self.GeometryCollection`))
  (bind _radialfalloff (`self.RadialFalloff`))
  (if (`self.ActorHasTag` OtherActor "Plasma")
    (`/Engine/EditorBlueprintResources/StandardMacros.DoOnce` false
      (:`Completed`
        (`ActorComponent.K2_DestroyComponent` (`self.StaticMesh`))
        (`SceneComponent.SetHiddenInGame` _geometrycollection false false)
        (`PrimitiveComponent.SetSimulatePhysics` _geometrycollection true)
        (bind _output_get (set `RadialFalloff.Position` (`KismetMathLibrary.InverseTransformLocation` (`self.GetTransform`) (`.Location` (`GameplayStatics.BreakHitResult` Hit))) _radialfalloff))
        (`FieldSystemComponent.ApplyPhysicsField` (`self.FieldSystem`) true "Field_ExternalClusterStrain" null _radialfalloff)
        (`KismetSystemLibrary.DrawDebugSphere` _output_get (`RadialFalloff.Radius` _radialfalloff) 12 (struct :`R` 1.0 :`G` 1.0 :`B` 1.0 :`A` 1.0) 1.0 1.0)))))

(fn `UserConstructionScript`)